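; BP_Floater is an actor that bobs up and down around the position where it begins play.
; BeginPlay stores the start location, and each Tick accumulates running time and sets the Z to the start height plus a sine wave scaled by Amplitude and Frequency.
; X and Y stay fixed at the start values.
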(event `self.ReceiveBeginPlay`
  (set `self.StartLocation` (`self.K2_GetActorLocation`)))

(event `self.ReceiveTick`
  (params (DeltaSeconds :type "Float (single-precision)"))
  (bind (_startlocation_x _startlocation_y _startlocation_z) (`KismetMathLibrary.BreakVector` (`self.StartLocation`)))
  (set `self.RunningTime` (+ (`self.RunningTime`) DeltaSeconds))
  (`self.K2_SetActorLocation` (`KismetMathLibrary.MakeVector` _startlocation_x _startlocation_y (+ _startlocation_z (* (`self.Amplitude`) (`KismetMathLibrary.Sin` (* (`self.Frequency`) (`self.RunningTime`))))))))

(fn `UserConstructionScript`)