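; Pianist ghost character that, once submitted to, plays its level sequence and takes up the piano.
; Instrument and bowtie start hidden; Submit starts PianistSequence, unlocks the kitchen door and teleports the ghost high out of the way.
; A Tick-polled flag and 5.1-second delay then place it at its final spot, show both props and start the music manager's piano.
; The flag never resets, so that step repeats after each delay.
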(event `self.ReceiveBeginPlay`
  (`parent.ReceiveBeginPlay`)
  (set `self.sequenceDone` false)
  (`SceneComponent.SetVisibility` (`self.instrument`) false false)
  (`SceneComponent.SetVisibility` (`self.bowtie`) false false))

(event `self.ReceiveTick`
  (params (DeltaSeconds :type "Float (single-precision)"))
  (`parent.ReceiveTick` DeltaSeconds)
  (if (`self.sequenceDone`)
    (`KismetSystemLibrary.Delay` 5.1)
    (`self.K2_SetActorLocation` (1770.0 1450.0 -4.0) false true)
    (`self.K2_SetActorRotation` (struct :`Yaw` 100.0))
    (`self.Talk` "")
    (`SceneComponent.SetVisibility` (`self.instrument`) true false)
    (`SceneComponent.SetVisibility` (`self.bowtie`) true false)
    (bind _outactors (`GameplayStatics.GetAllActorsOfClassWithTag` "/Game/_MyContent/BP_MusicManager.BP_MusicManager_C" "music"))
    (`/Game/_MyContent/BP_MusicManager.BeginPiano` (`|GetArrayItem` _outactors))))

(fn `Submit`
  (`parent.Submit`)
  (bind _outactor (`LevelSequencePlayer.CreateLevelSequencePlayer` "/Game/_MyContent/Sequences/PianistSequence.PianistSequence"))
  (`MovieSceneSequencePlayer.Play` (`LevelSequenceActor.SequencePlayer` _outactor))
  (bind _outactors (`GameplayStatics.GetAllActorsOfClassWithTag` "/Game/_MyContent/BP_DoorLock.BP_DoorLock_C" "kitchen"))
  (`/Game/_MyContent/BP_DoorLock.Unlock` (`|GetArrayItem` _outactors))
  (`self.K2_SetActorLocation` (1622.8 1342.23 2000.0) false true)
  (set `self.sequenceDone` true))

(fn `Talk_0`
  (locals (NewLocalVar :type Boolean)))

(fn `UserConstructionScript`
  (`parent.UserConstructionScript`))