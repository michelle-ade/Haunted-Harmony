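; BP_Stand is a stand actor with a static mesh, box and widget that detects overlap with the third-person player character.
; On BeginPlay it hides the mesh and widget, enlarges the box from the mesh bounds, and moves its root to a hardcoded world location.
; Actor overlap only prints debug text reporting a player hit or a failed character cast.
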(event `self.ReceiveBeginPlay`
  (`SceneComponent.SetVisibility` (`self.StaticMesh`) false false)
  (`SceneComponent.SetVisibility` (`self.Widget`) false false)
  (`BoxComponent.SetBoxExtent` (`self.Box`) (* (`.BoxExtent` (`KismetSystemLibrary.GetComponentBounds` (`self.StaticMesh`))) (1.4 1.4 1.4)) true)
  (`SceneComponent.K2_SetWorldLocation` (`self.DefaultSceneRoot`) (1232.855839 1308.848147 2500.0) false false))

(event `self.ReceiveActorBeginOverlap`
  (params (OtherActor :type "Actor Object Reference"))
  (cast `/Game/ThirdPerson/Blueprints/BP_ThirdPersonCharacter` OtherActor
    (:`then`
      (`KismetSystemLibrary.PrintString` "stand hit player"))
    (:`CastFailed`
      (`KismetSystemLibrary.PrintString` "character cast failed"))))

(fn `UserConstructionScript`)