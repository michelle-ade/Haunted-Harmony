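; BP_Ghost is a ghost NPC that waits for the player to bring a required item.
; On BeginPlay it sizes a trigger box slightly beyond the mesh bounds and hides its floating-text widget.
; On overlap it string-compares the character's HeldItem to RequiredItemTxt; a match sets ConditionMet and Talk displays SubmitTxt.
; Submit, intended for receiving the item and moving to stage, only talks and prints, and is not called here.
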(event `self.ReceiveBeginPlay`
  (set `self.ConditionMet` false)
  (`BoxComponent.SetBoxExtent` (`self.Box`) (* (`.BoxExtent` (`KismetSystemLibrary.GetComponentBounds` (`self.StaticMesh`))) (1.4 1.4 1.4)) true)
  (`Widget.SetVisibility` (`WidgetComponent.GetUserWidgetObject` (`self.Widget`)) "Hidden"))

(event `self.ReceiveActorBeginOverlap`
  (params (OtherActor :type "Actor Object Reference"))
  (bind _returnvalue (`KismetTextLibrary.Conv_TextToString` (`self.requiredItemTxt`)))
  (bind _asbp_third_person_character (cast `/Game/ThirdPerson/Blueprints/BP_ThirdPersonCharacter` OtherActor)
    (:`then`
      (bind _returnvalue_2 (`KismetTextLibrary.Conv_TextToString` (`/Game/ThirdPerson/Blueprints/BP_ThirdPersonCharacter.heldItem` _asbp_third_person_character)))
      (if (== _returnvalue_2 _returnvalue)
        (set `self.ConditionMet` true)
        (`KismetSystemLibrary.PrintString` "ghost condition met")
        (`self.Talk` (`self.submitTxt`))
        (else
          (`KismetSystemLibrary.PrintString` "ghost condition not met")
          (`KismetSystemLibrary.PrintString` _returnvalue_2)
          (`KismetSystemLibrary.PrintString` _returnvalue))))
    (:`CastFailed`
      (`KismetSystemLibrary.PrintString` "character cast failed"))))

(fn `Submit`
  ;[1 1 1] receive item and move to stage
  (`self.Talk` (`self.submitTxt`))
  (`KismetSystemLibrary.PrintString` "going to stage"))

(fn `Talk`
  (params (Dialogue :type Text))
  (bind _aswbp_floating_text (cast `/Game/_MyContent/WBP_FloatingText` (`WidgetComponent.GetUserWidgetObject` (`self.Widget`)))
    (:`then`
      (`/Game/_MyContent/WBP_FloatingText.SetText` _aswbp_floating_text Dialogue)
      (`Widget.SetVisibility` (`WidgetComponent.GetUserWidgetObject` (`self.Widget`)) "Visible"))
    (:`CastFailed`
      (`KismetSystemLibrary.PrintString` "WBP cast failed"))))

(fn `UserConstructionScript`)