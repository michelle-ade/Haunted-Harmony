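; BP_Item is an item actor built around a StaticMesh and a Box component.
; On BeginPlay it fits the Box to the mesh's bounds, enlarged by a margin, so the volume follows whatever mesh is set.
; HideSelf disables actor collision and hides both components without destroying the actor.
; No overlap logic is implemented here, and a few debug and mesh-setting nodes are left disconnected.
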(event `self.ReceiveBeginPlay`
  (`BoxComponent.SetBoxExtent` (`self.Box`) (* (`.BoxExtent` (`KismetSystemLibrary.GetComponentBounds` (`self.StaticMesh`))) (1.4 1.4 1.4)) false))

(event `self.ReceiveTick`
  (params (DeltaSeconds :type "Float (single-precision)")))

(fn `hideSelf`
  (`self.SetActorEnableCollision` false)
  (`SceneComponent.SetVisibility` (`self.Box`) false false)
  (`SceneComponent.SetVisibility` (`self.StaticMesh`) false false))

(fn `UserConstructionScript`)