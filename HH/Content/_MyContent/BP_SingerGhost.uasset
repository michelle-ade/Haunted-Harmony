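; BP_SingerGhost is a singer ghost with a cage that hides on overlap once its condition is met.
; Submit plays the singer level sequence, unlocks the lounge door, lifts the ghost to a higher position and sets SequenceDone.
; Tick polls that flag and, after a delay, teleports the ghost back down, calls Talk, moves the tagged stand and starts vocals on the music manager.
; The flag is never cleared after Submit, so this repeats.
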(event `self.ReceiveBeginPlay`
  (`parent.ReceiveBeginPlay`)
  (set `self.sequenceDone` false))

(event `self.ReceiveActorBeginOverlap`
  (params (OtherActor :type "Actor Object Reference"))
  (`parent.ReceiveActorBeginOverlap` OtherActor)
  (if (`self.ConditionMet`)
    (`SceneComponent.SetVisibility` (`self.cage`) false false)))

(event `self.ReceiveTick`
  (params (DeltaSeconds :type "Float (single-precision)"))
  (`parent.ReceiveTick` DeltaSeconds)
  (if (`self.sequenceDone`)
    (`KismetSystemLibrary.Delay` 5.1)
    (`self.K2_SetActorLocation` (1516.0 1285.0 -9.54) false true)
    (`self.K2_SetActorRotation` (struct :`Yaw` 100.0))
    (`self.Talk` "")
    (bind _outactors (`GameplayStatics.GetAllActorsOfClassWithTag` "/Game/_MyContent/BP_Stand.BP_Stand_C" "stand"))
    (`SceneComponent.K2_SetWorldLocation` (`Actor.RootComponent` (`|GetArrayItem` _outactors)) (1232.855839 1308.848147 -89.479643) false false)
    (bind _outactors_2 (`GameplayStatics.GetAllActorsOfClassWithTag` "/Game/_MyContent/BP_MusicManager.BP_MusicManager_C" "music"))
    (`/Game/_MyContent/BP_MusicManager.BeginVocals` (`|GetArrayItem` _outactors_2))))

(fn `Submit`
  (`parent.Submit`)
  (bind _outactor (`LevelSequencePlayer.CreateLevelSequencePlayer` "/Game/_MyContent/Sequences/SingerSequence.SingerSequence"))
  (`MovieSceneSequencePlayer.Play` (`LevelSequenceActor.SequencePlayer` _outactor))
  (bind _outactors (`GameplayStatics.GetAllActorsOfClassWithTag` "/Game/_MyContent/BP_DoorLock.BP_DoorLock_C" "lounge"))
  (`/Game/_MyContent/BP_DoorLock.Unlock` (`|GetArrayItem` _outactors))
  (`self.K2_SetActorLocation` (1516.45 1285.565 1000.0) false true)
  (set `self.sequenceDone` true))

(fn `Talk_0`
  (locals (NewLocalVar :type Boolean)))

(fn `UserConstructionScript`
  (`parent.UserConstructionScript`))