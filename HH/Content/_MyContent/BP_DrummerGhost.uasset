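; Drummer ghost character that, on submission, plays its level sequence and unlocks the lounge door.
; Submit extends the parent, moves the ghost to the world origin and sets a done flag that Tick polls.
; After a roughly five-second Delay, Tick places the ghost at a hard-coded spot, calls Talk, reveals its instrument and starts the tagged music manager.
; The flag is never cleared, so that delayed block keeps repeating.
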(event `self.ReceiveBeginPlay`
  (`parent.ReceiveBeginPlay`)
  (set `self.sequenceDone` false)
  (`SceneComponent.SetVisibility` (`self.instrument`) false false))

(event `self.ReceiveTick`
  (params (DeltaSeconds :type "Float (single-precision)"))
  (`parent.ReceiveTick` DeltaSeconds)
  (if (`self.sequenceDone`)
    (`KismetSystemLibrary.Delay` 5.1)
    (`self.K2_SetActorLocation` (1876.973999 1029.965454 14.350168) false true)
    (`self.K2_SetActorRotation` (struct :`Yaw` 100.0))
    (`self.Talk` "")
    (`SceneComponent.SetVisibility` (`self.instrument`) true false)
    (bind _outactors (`GameplayStatics.GetAllActorsOfClassWithTag` "/Game/_MyContent/BP_MusicManager.BP_MusicManager_C" "music"))
    (`/Game/_MyContent/BP_MusicManager.StartMusic` (`|GetArrayItem` _outactors))))

(fn `Submit`
  (`parent.Submit`)
  (`GameplayStatics.GetActorOfClass` "/Script/Engine.LevelScriptActor")
  (bind _outactor (`LevelSequencePlayer.CreateLevelSequencePlayer` "/Game/_MyContent/Sequences/DrummerSequence.DrummerSequence"))
  (`MovieSceneSequencePlayer.Play` (`LevelSequenceActor.SequencePlayer` _outactor))
  (bind _outactors (`GameplayStatics.GetAllActorsOfClassWithTag` "/Game/_MyContent/BP_DoorLock.BP_DoorLock_C" "lounge"))
  (`/Game/_MyContent/BP_DoorLock.Unlock` (`|GetArrayItem` _outactors))
  (`self.K2_SetActorLocation` (0.0 0.0 0.0) false true)
  (set `self.sequenceDone` true))

(fn `Talk_0`
  (locals (NewLocalVar :type Boolean)))

(fn `UserConstructionScript`
  (`parent.UserConstructionScript`))